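; Yin E ability ranged hit actor that damages the first valid character it overlaps, ignoring its instigator, then destroys itself.
; End and Capsule overlaps share one path: the server line-traces Start to End for a hit result, while clients just destroy the actor.
; The target's own ASC builds and self-applies the basic-attack damage effect with SetByCaller magnitude and hit context.
; Lifespan scales inversely with a Yin attribute.
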(event `self.ReceiveBeginPlay`
  (bind _asyin_player_character_2 (cast `/Game/RaidCharacter/Yin/YinPlayerCharacter_2` (`self.GetInstigator`))
    (:`then`
      (`self.SetLifeSpan` (/ 1.2 (`.ReturnValue` (`AbilitySystemBlueprintLibrary.GetFloatAttribute` _asyin_player_character_2 (struct :`AttributeName` "AttackSpeed" :`Attribute` "/Script/RaidGame.BaseAttributeSet:AttackSpeed" :`AttributeOwner` "/Script/CoreUObject.Class'/Script/RaidGame.BaseAttributeSet'"))))))
    (:`CastFailed`
      (`self.SetLifeSpan` 1.0))))

(event `self.End.OnComponentBeginOverlap`
  (params (OverlappedComponent :type "PrimitiveComponent Object Reference") (OtherActor :type "Actor Object Reference") (OtherComp :type "PrimitiveComponent Object Reference") (OtherBodyIndex :type Integer) (bFromSweep :type Boolean) (SweepResult :type "HitResult Structure (by ref)"))
  (if (!= OtherActor (`self.GetInstigator`)) :!label _label
    (`/Engine/EditorBlueprintResources/ActorMacros.Switch Has Authority`
      (:`Authority`
        (bind _asbase_character (cast `BaseCharacter` OtherActor))
        (bind _returnvalue (`AbilitySystemBlueprintLibrary.GetAbilitySystemComponent` _asbase_character))
        (if (`KismetSystemLibrary.IsValid` _returnvalue)
          (bind _outhits (`KismetSystemLibrary.LineTraceMultiForObjects` :`Start` (`SceneComponent.K2_GetComponentLocation` (`self.Start`)) :`End` (`SceneComponent.K2_GetComponentLocation` (`self.End`)) :`ObjectTypes` (`|MakeArray` "ObjectTypeQuery3" :!type "EObjectTypeQuery Enum") :`DrawTime` 2.0))
          (for _array_element _outhits
            (if (== (`.HitActor` (`GameplayStatics.BreakHitResult` _array_element)) _asbase_character)
              (set `self.Final Hit` _array_element)
              (break)))
          (bind _returnvalue_2 (`AbilitySystemBlueprintLibrary.AssignTagSetByCallerMagnitude` (`AbilitySystemComponent.MakeOutgoingSpec` :`self` _returnvalue :`GameplayEffectClass` "/Game/RaidCharacter/Yin/Yin_Ability/Yin_A_Ability/GE_Yin_A_BasicAttack_Damage.GE_Yin_A_BasicAttack_Damage_C") (struct :`TagName` "SetByCaller.Damage") (`self.Damage`)))
          (bind _returnvalue_3 (`AbilitySystemBlueprintLibrary.GetEffectContext` _returnvalue_2))
          (`AbilitySystemBlueprintLibrary.EffectContextAddHitResult` _returnvalue_3 (`self.Final Hit`))
          (`AbilitySystemComponent.BP_ApplyGameplayEffectSpecToSelf` _returnvalue _returnvalue_2)
          (`self.K2_DestroyActor`)))
      (:`Remote`
        (`self.K2_DestroyActor`)))))

(event `self.Capsule.OnComponentBeginOverlap`
  (params (OverlappedComponent :type "PrimitiveComponent Object Reference") (OtherActor :type "Actor Object Reference") (OtherComp :type "PrimitiveComponent Object Reference") (OtherBodyIndex :type Integer) (bFromSweep :type Boolean) (SweepResult :type "HitResult Structure (by ref)"))
  (goto _label))

(event `self.StaticMesh.OnComponentBeginOverlap`
  (params (OverlappedComponent :type "PrimitiveComponent Object Reference") (OtherActor :type "Actor Object Reference") (OtherComp :type "PrimitiveComponent Object Reference") (OtherBodyIndex :type Integer) (bFromSweep :type Boolean) (SweepResult :type "HitResult Structure (by ref)")))

(fn `UserConstructionScript`)