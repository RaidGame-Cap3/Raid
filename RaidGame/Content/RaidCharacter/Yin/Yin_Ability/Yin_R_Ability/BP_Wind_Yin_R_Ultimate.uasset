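; Wind area actor for Yin's R ultimate that grants a buff, noted as temporary armor, to player characters inside its sphere.
; When a Pawn enters, the server applies GE_Wind_Buff_Yin_R_UltimateAbility to every living overlapping PlayerCharacter with an ability system component.
; The overlap also leads to a delay of ActorActiveTime before the actor destroys itself, so its removal timer depends on an overlap rather than on spawn.
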(event `self.Sphere.OnComponentBeginOverlap`
  (params (OverlappedComponent :type "PrimitiveComponent Object Reference") (OtherActor :type "Actor Object Reference") (OtherComp :type "PrimitiveComponent Object Reference") (OtherBodyIndex :type Integer) (bFromSweep :type Boolean) (SweepResult :type "HitResult Structure (by ref)"))
  ;[1 1 1] 충돌 개체가 Pawn이면
  (if (`|EnumEquality` (`PrimitiveComponent.GetCollisionObjectType` OtherComp) "ECC_Pawn")
    ;[0 0.9519 1] 서버인 경우에만 효과 적용.
    ; 다른 것에 미치는 영향 예측 X
    (`/Engine/EditorBlueprintResources/ActorMacros.Switch Has Authority`
      (:`Authority`
        (for _array_element (`PrimitiveComponent.GetOverlappingActors` (`self.Sphere`) "/Script/RaidGame.BaseCharacter")
          (bind _asplayer_character (cast `PlayerCharacter` _array_element))
          (bind _returnvalue (`AbilitySystemBlueprintLibrary.GetAbilitySystemComponent` _asplayer_character))
          (if (and (`BaseCharacter.IsAlive` _asplayer_character) (`KismetSystemLibrary.IsValid` _returnvalue))
            ;[0.5878 0.5334 0.7656] PlayerCharacter를 가진 instigator 충돌 간에 아머 적용
            ; 5초간 지속되는 아머 수치를 30으로 조정
            (bind _output_get (set `self.ArmorEffectSpecHandle` (`AbilitySystemComponent.MakeOutgoingSpec` :`self` _returnvalue :`GameplayEffectClass` "/Game/RaidCharacter/Yin/Yin_Ability/Yin_R_Ability/GE_Wind_Buff_Yin_R_UltimateAbility.GE_Wind_Buff_Yin_R_UltimateAbility_C")))
            (`AbilitySystemComponent.BP_ApplyGameplayEffectSpecToSelf` _returnvalue _output_get))))
      (:`Remote`
        _))
    ;[1 1 1] 일정 시간 후 액터 제거
    (`KismetSystemLibrary.Delay` (`self.ActorActiveTime`))
    (`self.K2_DestroyActor`)))

(fn `UserConstructionScript`)