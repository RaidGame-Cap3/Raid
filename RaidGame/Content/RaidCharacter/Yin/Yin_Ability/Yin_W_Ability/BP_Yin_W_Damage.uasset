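; Damage actor for Yin's W ability that hurts characters inside its sphere when a pawn begins overlapping it.
; On the server, it sweeps all overlapping BaseCharacters except the instigator and applies GE_Yin_W_Ability2_Damage with SetByCaller damage.
; Each spec is made and self-applied through the target's own ability system component, not the instigator's.
; The server destroys the actor after a short delay, while remotes destroy it immediately without predicting damage.
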(event `self.Sphere.OnComponentBeginOverlap`
  (params (OverlappedComponent :type "PrimitiveComponent Object Reference") (OtherActor :type "Actor Object Reference") (OtherComp :type "PrimitiveComponent Object Reference") (OtherBodyIndex :type Integer) (bFromSweep :type Boolean) (SweepResult :type "HitResult Structure (by ref)"))
  (if (`|EnumEquality` (`PrimitiveComponent.GetCollisionObjectType` OtherComp) "ECC_Pawn")
    ;[0 0.9519 1] 서버인 경우에만 효과 적용.
    ; 다른 것에 미치는 영향 예측 X
    (`/Engine/EditorBlueprintResources/ActorMacros.Switch Has Authority`
      (:`Authority`
        (for _array_element (`PrimitiveComponent.GetOverlappingActors` (`self.Sphere`) "/Script/RaidGame.BaseCharacter")
          (bind _asbase_character (cast `BaseCharacter` _array_element))
          (bind _returnvalue (`AbilitySystemBlueprintLibrary.GetAbilitySystemComponent` _asbase_character))
          (if (and (not (== _asbase_character (`self.GetInstigator`))) (`KismetSystemLibrary.IsValid` _returnvalue))
            ;[0.2513 0.2868 0.3125] 자신을 제외한 BaseCharacter를 가진 액터들에게
            ;  Damage 만큼 체력 감소하는 이펙트 부여
            ; 추후 몬스터에게만 적용되도록 변경 예정
            (bind _returnvalue_2 (`AbilitySystemBlueprintLibrary.AssignTagSetByCallerMagnitude` (`AbilitySystemComponent.MakeOutgoingSpec` :`self` _returnvalue :`GameplayEffectClass` "/Game/RaidCharacter/Yin/Yin_Ability/Yin_W_Ability/GE_Yin_W_Ability2_Damage.GE_Yin_W_Ability2_Damage_C") (struct :`TagName` "SetByCaller.Damage") (`self.damage`)))
            (`AbilitySystemComponent.BP_ApplyGameplayEffectSpecToSelf` _returnvalue _returnvalue_2)))
        ;[1 1 1] 일정 시간 후 액터 제거
        (`KismetSystemLibrary.Delay` 0.5)
        (`self.K2_DestroyActor`))
      (:`Remote`
        (`self.K2_DestroyActor`)))))

(fn `UserConstructionScript`)