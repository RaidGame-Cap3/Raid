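; BP_Test_Enemy is a test enemy that uses the Gameplay Ability System for health and mana regeneration.
; On BeginPlay it applies the default health and mana regen GameplayEffects to itself through its Ability System Component.
; It then sets itself as OwnerActor on its HPBar component's Widget_Test_HPbar.
; Without a valid Ability System Component, it only prints an error and leaves the bar unbound.
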(event `self.ReceiveBeginPlay`
  (bind _returnvalue (`AbilitySystemBlueprintLibrary.GetAbilitySystemComponent` null))
  ;[0.5882 0.5333 0.7647] 체력 및 마나 자동 회복 로직
  ; Health 1초에 1씩 회복하여 MaxHealth(default=100)까지 오름
  ; Mana 3초에 5씩 회복하여 MaxMana(default=100)까지 오름
  (if (`KismetSystemLibrary.IsValid` _returnvalue)
    (`AbilitySystemComponent.BP_ApplyGameplayEffectToSelf` :`self` _returnvalue :`GameplayEffectClass` "/Game/RaidCharacter/default/GE_Default_Health_Regen.GE_Default_Health_Regen_C")
    (`AbilitySystemComponent.BP_ApplyGameplayEffectToSelf` :`self` _returnvalue :`GameplayEffectClass` "/Game/RaidCharacter/default/GE_Default_Mana_Regen.GE_Default_Mana_Regen_C")
    (bind _aswidget_test_hpbar (cast `/Game/RaidCharacter/Test/Widget_Test_HPbar` (`WidgetComponent.GetUserWidgetObject` (`self.HPBar`))))
    (set `/Game/RaidCharacter/Test/Widget_Test_HPbar.ownerActor` self _aswidget_test_hpbar)
    (else
      (`KismetSystemLibrary.PrintString` "어빌리티 컴포넌트를 가져오지 못했습니다."))))

(fn `UserConstructionScript`)