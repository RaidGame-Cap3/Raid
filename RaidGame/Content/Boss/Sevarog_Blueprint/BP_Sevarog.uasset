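; Sevarog boss Blueprint that turns toward the player and performs swing, shooting-ball, tornado and laser attacks.
; Tick feeds a five-second Delay into an attack switch, but the random range is pinned so only the tornado case runs.
; Each attack toggles timed state booleans, with swing, shot and laser spawning actors at mesh sockets.
; The tornado spawn targets the player's location but has no class set.
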(event `self.ReceiveTick`
  (params (DeltaSeconds :type "Float (single-precision)"))
  (bind (_returnvalue_roll _returnvalue_pitch _returnvalue_yaw) (`KismetMathLibrary.BreakRotator` (`KismetMathLibrary.FindLookAtRotation` (`self.K2_GetActorLocation`) (`self.K2_GetActorLocation` (`GameplayStatics.GetPlayerCharacter` 0)))))
  (bind (_returnvalue_roll_2 _returnvalue_pitch_2 _returnvalue_yaw_2) (`KismetMathLibrary.BreakRotator` (`KismetMathLibrary.FindLookAtRotation` (`self.K2_GetActorLocation`) (`self.K2_GetActorLocation` (`GameplayStatics.GetPlayerCharacter` 0)))))
  (bind (_returnvalue_roll_3 _returnvalue_pitch_3 _returnvalue_yaw_3) (`KismetMathLibrary.BreakRotator` (`KismetMathLibrary.FindLookAtRotation` (`self.K2_GetActorLocation`) (`self.K2_GetActorLocation` (`GameplayStatics.GetPlayerCharacter` 0)))))
  (bind (_returnvalue_roll_4 _returnvalue_pitch_4 _returnvalue_yaw_4) (`KismetMathLibrary.BreakRotator` (`KismetMathLibrary.FindLookAtRotation` (`self.K2_GetActorLocation`) (`self.K2_GetActorLocation` (`GameplayStatics.GetPlayerCharacter` 0)))))
  (`KismetSystemLibrary.Delay` 5.0)
  (switch `int` (`KismetMathLibrary.RandomIntegerInRange` 3 3)
    (:`1`
      ;[1 1 1] Swing Attack
      (`self.K2_SetActorRotation` (`KismetMathLibrary.MakeRotator` 0.0 0.0 _returnvalue_yaw_2))
      (set `self.SwingAttack` true)
      (`KismetSystemLibrary.Delay` 0.1)
      (`|SpawnActorFromClass` "/Game/Boss/Actors/BlackBall.BlackBall_C" (`KismetMathLibrary.MakeTransform` (`SceneComponent.GetSocketLocation` (`self.SkeletalMesh_Sevarog`) "HammerCenter") (`self.K2_GetActorRotation`) (`self.GetActorScale3D`)) "Undefined" "MultiplyWithRoot" null null)
      (`KismetSystemLibrary.Delay` 0.9)
      (`|ExecutionSequence`
        (:`then_0`
          (set `self.SwingAttack` false))
        (:`then_1`
          (set `self.SwingReturn` true)
          (`KismetSystemLibrary.Delay` 2.1)
          (set `self.SwingReturn` false))))
    (:`2`
      ;[1 1 1] ShootingBall
      (`self.K2_SetActorRotation` (`KismetMathLibrary.MakeRotator` 0.0 0.0 _returnvalue_yaw_3))
      (set `self.ShootingBall` true)
      (`KismetSystemLibrary.Delay` 0.1)
      (`|ExecutionSequence`
        (:`then_0`
          (`|SpawnActorFromClass` "/Game/Boss/Actors/TestActor.TestActor_C" (`KismetMathLibrary.MakeTransform` (`SceneComponent.GetSocketLocation` (`self.SkeletalMesh_Sevarog`) "FX_Head") (`self.K2_GetActorRotation`) (`self.GetActorScale3D`)) "Undefined" "MultiplyWithRoot" null null)
          (`KismetSystemLibrary.Delay` 1.2)
          (set `self.ShootingBall` false))
        (:`then_1`
          (`|SpawnActorFromClass` "/Game/Boss/Actors/TestActor.TestActor_C" (`KismetMathLibrary.MakeTransform` (`SceneComponent.GetSocketLocation` (`self.SkeletalMesh_Sevarog`) "ShoulderL_1") (`self.K2_GetActorRotation`) (`self.GetActorScale3D`)) "Undefined" "MultiplyWithRoot" null null))
        (:`then_2`
          (`|SpawnActorFromClass` "/Game/Boss/Actors/TestActor.TestActor_C" (`KismetMathLibrary.MakeTransform` (`SceneComponent.GetSocketLocation` (`self.SkeletalMesh_Sevarog`) "ShoulderR_1") (`self.K2_GetActorRotation`) (`self.GetActorScale3D`)) "Undefined" "MultiplyWithRoot" null null))))
    (:`3`
      ;[1 1 1] CastingTornado
      (`self.K2_SetActorRotation` (`KismetMathLibrary.MakeRotator` 0.0 0.0 _returnvalue_yaw_4))
      (set `self.CastingTornado` true)
      (`KismetSystemLibrary.Delay` 1.0)
      (`|SpawnActorFromClass` "/Game/Boss/Actors/tornado.tornado_C" (`KismetMathLibrary.Conv_VectorToTransform` (`self.K2_GetActorLocation` (`GameplayStatics.GetPlayerCharacter` 0))) "Undefined" "MultiplyWithRoot" null null)
      (`KismetSystemLibrary.Delay` 1.6)
      (set `self.CastingTornado` false))
    (:`4`
      ;[1 1 1] CastingLaser
      (`self.K2_SetActorRotation` (`KismetMathLibrary.MakeRotator` 0.0 0.0 _returnvalue_yaw))
      (set `self.CastingLaser` true)
      (`KismetSystemLibrary.Delay` 0.9)
      (`|SpawnActorFromClass` "/Game/Boss/Actors/BlackBall.BlackBall_C" (`KismetMathLibrary.MakeTransform` (`SceneComponent.GetSocketLocation` (`self.SkeletalMesh_Sevarog`) "Hand_L_Cast") (`self.K2_GetActorRotation`) (`self.GetActorScale3D`)) "Undefined" "MultiplyWithRoot" null null)
      (`KismetSystemLibrary.Delay` 2.2)
      (`|ExecutionSequence`
        (:`then_0`
          (set `self.CastingLaser` false))
        (:`then_1`
          (set `self.LaserLoop` true)
          (`KismetSystemLibrary.Delay` 0.2)
          (set `self.LaserLoop` false))))))

(fn `UserConstructionScript`)